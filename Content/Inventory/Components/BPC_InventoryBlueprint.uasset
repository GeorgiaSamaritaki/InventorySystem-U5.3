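; Inventory component that lets the player pick up world items and view them in an inventory widget.
; Each tick, a sphere trace ahead of the character toggles the pickup prompt, and the pickup input reruns it, destroying the actor once its item is stored.
; Adding stacks items up to DT_Items stack limits or fills empty slots in fixed-size arrays, with only Food handled, then refreshes the UI.
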(event EventBeginPlay
  (Input|AddMappingContext (PlayerController|LocalPlayerSubsystems|GetEnhancedInputLocalPlayerSubsystem (Game|GetPlayerController 0)) "/Game/Inventory/Inputs/IMC_InventoryInput.IMC_InventoryInput" 0 "(bIgnoreAllPressedKeysUntilRelease=True,bForceImmediately=False,bNotifyUserSettings=False)")
  (bind _returnvalue (UserInterface|CreateWidget 0))
  (Variables|Widgets|SetWBP_Inventory 0 _returnvalue)
  (bind _asbp_third_person_character (Utilities|Casting|CastToBP_ThirdPersonCharacter (Game|GetPlayerCharacter 0)))
  (Variables|Default|SetAs%20BP%20Third%20Person%20Character _asbp_third_person_character)
  (bind _returnvalue_2 (UserInterface|CreateWidget "/Game/Inventory/Widgets/WBP_PickUp.WBP_PickUp_C"))
  (Variables|Widgets|SetWBP_PickUp _returnvalue_2)
  (CallFunction|UpdateInventorySize)
  (CallFunction|UpdateItemsinInventoryUI (.WBP_Inventory (Variables|Widgets|GetWBP_Inventory)) (Variables|Default|GetAllItem)))

(event EventTick
  (params (DeltaSeconds :type Float%20%28single-precision%29))
  (bind _founditem (CallFunction|DetectItemtoPickUp))
  (Utilities|ShowPickupWidget _founditem))

(event Input|EnhancedActionEvents|EnhancedInputActionIA_PickUp
  (params (ActionValue :type Boolean) (ElapsedSeconds :type Float%20%28double-precision%29) (TriggeredSeconds :type Float%20%28double-precision%29) (InputAction :type Input%20Action%20Object%20Reference :default "/Game/Inventory/Inputs/IA_PickUp.IA_PickUp"))
  ;[0.05208 0.05208 0.05208 0.895] Add to Inventory
  (bind (_item _founditem _itemactor) (CallFunction|DetectItemtoPickUp))
  (if _founditem
    (bind _success (CallFunction|AddtoInventory _item))
    (if _success
      (Actor|DestroyActor _itemactor))))

(event Input|EnhancedActionEvents|EnhancedInputActionIA_Inventory
  (params (ActionValue :type Boolean) (ElapsedSeconds :type Float%20%28double-precision%29) (TriggeredSeconds :type Float%20%28double-precision%29) (InputAction :type Input%20Action%20Object%20Reference :default "/Game/Inventory/Inputs/IA_Inventory.IA_Inventory"))
  (bind _returnvalue (Game|GetPlayerController 0))
  ;[0.05208 0.05208 0.05208 0.895] Open Inventory
  (UserInterface|Viewport|AddtoViewport (.WBP_Inventory (Variables|Widgets|GetWBP_Inventory)) 0)
  (Variables|/Script/Engine.PlayerController|SetbShowMouseCursor _returnvalue true)
  (Input|SetInputModeUIOnly _returnvalue (.WBP_Inventory (Variables|Widgets|GetWBP_Inventory)) "DoNotLock" false))

(fn DetectItemtoPickUp
  (bind _returnvalue (Game|GetPlayerCharacter 0))
  (bind _returnvalue_2 (Transformation|GetActorLocation _returnvalue))
  (bind _returnvalue_3 (- _returnvalue_2 "0.000000,0.000000,60.000000"))
  (bind _outhit (Collision|SphereTraceByChannel _returnvalue_3 (+ _returnvalue_3 (* (Transformation|GetActorForwardVector _returnvalue) 1.5e+02)) 3e+01 "TraceTypeQuery1" true 0 "ForOneFrame"))
  (bind _asbp_itemm (Utilities|Casting|CastTo (.hitactor _outhit))
    (:then
      (return (Variables|Default|GetItem _asbp_itemm) true (.hitactor _outhit)))
    (:CastFailed
      (return "" false 0))))

(fn AddtoInventory
  (params (Item :type Fallback%20Struct%20Structure%20%28by%20ref%29))
  (bind _allitem (Variables|Default|GetAllItem))
  (bind _food (Utilities|Struct|BreakFallbackStruct _allitem))
  (switch Utilities|FlowControl|Switch|Switchon (.ItemType (Utilities|Struct|BreakFallbackStruct Item))
    (:NewEnumerator0
      (for (_ _array_index) _food
        (bind _success (CallFunction|AddItemtoIndex Item _array_index _food))
        (if _success
          (CallFunction|UpdateUI)
          (return true)))
      ;[0.2552 0.2552 0.2552 0.68] Create new stack in inventory
      (for (_array_element _array_index_2) (Utilities|Struct|BreakFallbackStruct (Variables|Default|GetAllItem))
        (if (== (.Quantity (Utilities|Struct|BreakFallbackStruct _array_element)) 0)
          (Utilities|Array|SetArrayElem (Utilities|Struct|BreakFallbackStruct (Variables|Default|GetAllItem)) _array_index_2 Item)
          (CallFunction|UpdateUI)
          (return true)))
      (return false))))

(fn UpdateInventorySize
  (Utilities|Array|Resize (Utilities|Struct|BreakFallbackStruct (Variables|Default|GetAllItem)) (Variables|Default|GetInventorySize))
  (CallFunction|UpdateUI))

(fn UpdateUI
  (CallFunction|UpdateItemsinInventoryUI (.WBP_Inventory (Variables|Widgets|GetWBP_Inventory)) (Variables|Default|GetAllItem)))

(fn AddItemtoIndex
  (params (Item :type Fallback%20Struct%20Structure%20%28by%20ref%29) (Index :type Integer) (Array :type Array%20of%20Fallback%20Struct%20Structures))
  (bind (_itemid _itemtype _quantity) (Utilities|Struct|BreakFallbackStruct Item))
  (bind _output (Utilities|Array|Get(acopy) Array Index))
  (bind (_itemid_2 _itemtype_2 _quantity_2) (Utilities|Struct|BreakFallbackStruct _output))
  (bind (_itemid_3 _itemtype_3) (Utilities|Struct|BreakFallbackStruct Item))
  (bind _rowname (Utilities|Struct|BreakDataTableRowHandle _itemid_2))
  (bind _returnvalue (+ _quantity_2 _quantity))
  (if (or (== (.RowName (Utilities|Struct|BreakDataTableRowHandle _itemid)) _rowname) (== _quantity_2 0))
    (bind _returnvalue_2 (Utilities|GetDataTableRow "/Game/Inventory/Datastructures/DT_Items.DT_Items" _rowname)
      (:then
        (if (>= (.StackSize (Utilities|Struct|BreakItemRow _returnvalue_2)) _returnvalue)
          (Utilities|Array|SetArrayElem Array Index (Utilities|Struct|MakeFallbackStruct _itemid_3 _itemtype_3 _returnvalue))
          (CallFunction|UpdateUI)
          (return true)
          (else
            _)))
      (:RowNotFound
        _)))
  (return false))

(fn GetItemTypeArray
  (params (Selection :type Byte :default 0))
  (switch Utilities|FlowControl|Switch|Switchon Selection
    (:NewEnumerator0
      (return (Utilities|Struct|BreakFallbackStruct (Variables|Default|GetAllItem))))
    (:NewEnumerator1
      _)
    (:NewEnumerator2
      _))
  (return 0))

(fn PrintSlotArray
  (params (Array :type Array%20of%20Fallback%20Struct%20Structures))
  (for (_array_element _array_index) Array
    (Development|PrintString (Utilities|String|ToString(Text) (Utilities|Text|FormatText "Slot Array {Index} :{Name} {Quantity}" _array_index (.RowName (Utilities|Struct|BreakDataTableRowHandle (.ItemID (Utilities|Struct|BreakFallbackStruct _array_element)))) (.Quantity (Utilities|Struct|BreakFallbackStruct _array_element)))) true true "(R=0.000000,G=0.660000,B=1.000000,A=1.000000)" 15.0))
  (Development|PrintString "-------------" true true "(R=0.000000,G=0.660000,B=1.000000,A=1.000000)" 15.0)
  (return))

(fn PrintSlot
  (params (S_Slot :type Fallback%20Struct%20Structure%20%28by%20ref%29))
  (bind (_itemid _itemtype _quantity) (Utilities|Struct|BreakFallbackStruct S_Slot))
  (Development|PrintString (Utilities|String|ToString(Text) (Utilities|Text|FormatText "Item {Name} Quantity {Quantity}" (.RowName (Utilities|Struct|BreakDataTableRowHandle _itemid)) _quantity)))
  (return))